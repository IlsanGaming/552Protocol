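; Destructible, networked spotlight prop that breaks the first time it takes any damage.
; The damage event wakes net dormancy, forces an update, sets the destroyed flag, removes its health component and multicasts cosmetic effects.
; Destroy, also called from the flag's OnRep, waits a tick, removes the light, swaps the stand mesh and disables further damage.
; Sparks, impact particles and sound play only where cosmetic events can execute.
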(event Custom|Destroy
  ;[0 0 0] Destroy
  (Utilities|FlowControl|DelayUntilNextTick)
  (Components|DestroyComponent (Variables|Default|GetSpotLight))
  (Components|StaticMesh|SetStaticMesh (Variables|Default|GetSM_SpotlightStand) "/Game/FPS_Controller/Environment/Meshes/SM_Spotlight_03.SM_Spotlight_03")
  (Variables|Actor|SetbCanBeDamaged false))

(event Custom|Multicast_PlayCosmeticEffects
  (bind _sm_spotlightstand (Variables|Default|GetSM_SpotlightStand))
  (bind _returnvalue (Transformation|GetWorldLocation _sm_spotlightstand))
  ;[0 0 0] Play Effects
  (Networking|CanExecuteCosmeticEvents
    (:True
      (Niagara|SpawnSystematLocation "/Game/FPS_Controller/Effects/Particles/NS_Sparks.NS_Sparks" _returnvalue)
      (Effects|SpawnEmitteratLocation "/Game/FPS_Controller/Effects/Particles/P_RifleImpact.P_RifleImpact" _returnvalue "0, 0, 0" "5.000000,5.000000,5.000000")
      (Audio|PlaySoundatLocation 0 _returnvalue "0, 0, 0" 0.5 1.0 0.0 0 0 0 0))))

(event Game|Damage|EventAnyDamage
  (params (Damage :type Float%20%28single-precision%29) (DamageType :type Damage%20Type%20Object%20Reference) (InstigatedBy :type Controller%20Object%20Reference) (DamageCauser :type Actor%20Object%20Reference))
  ;[0 0 0] Any Damage
  (if (not (Variables|Default|GetbDestroyed))
    (Networking|SetNetDormancy "DORM_Awake")
    (Networking|ForceNetUpdate)
    (Variables|Default|SetbDestroyed true)
    (CallFunction|Destroy)
    (CallFunction|MulticastPlayCosmeticEffects)
    (Components|DestroyComponent (Variables|Default|GetAC_Health))))

(fn ConstructionScript)

(fn OnRepBDestroyed
  (CallFunction|Destroy))