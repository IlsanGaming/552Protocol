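; Frag grenade lethal for the FPS controller, handling cooking, throwing and dropping.
; Activate starts a fuse timer, plays the first-person equip animation and shows a cooking crosshair widget.
; Release throws from in front of the camera and dropping spawns at the third-person mesh, both passing the remaining fuse; overcooking detonates in hand.
; A server spawn event creates BP_FragGrenade along the upward-tilted control rotation and reduces inventory lethal ammo.
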(event Custom|ExplodeGrenade
  ;[0 0 0] Activate
  (if (not (Variables|Default|GetbReleased))
    (Widget|RemovefromParent (Variables|Default|GetLethalWidget))
    (CallFunction|ServerSpawnGrenade 0.01 (Transformation|GetWorldLocation (Variables|Default|GetTPP_Mesh)))))

(event Custom|Server_SpawnGrenade
  (params (TimeLeft :type Float%20%28double-precision%29) (SpawnLocation :type Vector))
  (bind _returnvalue (Components|GetOwner))
  (bind _returnvalue_2 (Components|GetOwner))
  (bind _returnvalue_3 (Actor|GetComponentbyClass _returnvalue "/Game/FPS_Controller/Blueprints/Components/AC_InventorySystem.AC_InventorySystem_C"))
  (bind _returnvalue_4 (Game|GetInstigatorController _returnvalue_2))
  (bind _returnvalue_5 (Pawn|GetControlRotation _returnvalue_4 :!class /Script/Engine.Controller))
  ;[0.1719 0 0] Server Spawn Grenade
  (bind _returnvalue_6 (Game|SpawnActorfromClass "/Game/FPS_Controller/Blueprints/Weapons/BP_FragGrenade.BP_FragGrenade_C" (Math|Transform|MakeTransform SpawnLocation (Math|Rotator|MakeRotator (.roll _returnvalue_5) (+ (.pitch _returnvalue_5) 15.0) (.yaw _returnvalue_5)) "1.000000,1.000000,1.000000") "Undefined" "OverrideRootScale" _returnvalue_4 TimeLeft (.AsPawn (Utilities|Casting|CastToPawn _returnvalue_2))))
  (Utilities|IsValid _returnvalue_6
    (:Is%20Valid
      (Utilities|IsValid _returnvalue_3
        (:Is%20Valid
          (Default|ReduceLethalAmmo _returnvalue_3))))))

(event Custom|Reset
  ;[0 0 0] Reset
  (Variables|Default|SetbReleased false)
  (Utilities|Time|ClearandInvalidateTimerbyHandle (Variables|Default|GetCookGrenadeTimer)))

(event EventActivate
  ;[0 0 0] Activate
  (CallFunction|Reset)
  (bind _returnvalue (Utilities|Time|SetTimerbyEvent (delegate Custom|ExplodeGrenade) 3.7))
  (Variables|Default|SetCookGrenadeTimer _returnvalue)
  (Components|Animation|PlayAnimation (Variables|Default|GetFPP_Mesh) (Variables|Default|GetEquipLethalAnimation) false)
  ;;[0 0 0] Cooking grenade crosshair
  (bind _returnvalue_2 (UserInterface|CreateWidget "/Game/FPS_Controller/UI/Lethal/WB_CookingGrenade.WB_CookingGrenade_C" (Game|GetPlayerController 0)))
  (bind _output_get (Variables|Default|SetLethalWidget _returnvalue_2))
  (UserInterface|Viewport|AddtoViewport _output_get 0))

(event EventReleaseLethal
  ;[0 0 0] Release Lethal
  (bind _asplayer_controller (Utilities|Casting|CastToPlayerController (Game|GetInstigatorController (Components|GetOwner))))
  (CallFunction|ServerSpawnGrenade (Utilities|Time|GetTimerRemainingTimebyHandle (Variables|Default|GetCookGrenadeTimer)) (Math|Vector|MakeVector (.X (Math|Vector|BreakVector (+ (Camera|GetCameraLocation (Variables|/Script/Engine.PlayerController|GetPlayerCameraManager _asplayer_controller)) (* (Transformation|GetActorForwardVector _asplayer_controller) 1e+02)))) (.Y (Math|Vector|BreakVector (+ (Camera|GetCameraLocation (Variables|/Script/Engine.PlayerController|GetPlayerCameraManager _asplayer_controller)) (* (Transformation|GetActorForwardVector _asplayer_controller) 1e+02)))) (+ (.Z (Math|Vector|BreakVector (+ (Camera|GetCameraLocation (Variables|/Script/Engine.PlayerController|GetPlayerCameraManager _asplayer_controller)) (* (Transformation|GetActorForwardVector _asplayer_controller) 1e+02)))) 3e+01))))

(event EventOnRelease
  ;[0 0 0] On Release
  (bind _lethalwidget (Variables|Default|GetLethalWidget)
    (:then
      (Widget|RemovefromParent _lethalwidget)
      (Variables|Default|SetbReleased true)
      (Utilities|Time|ClearandInvalidateTimerbyHandle (Variables|Default|GetCookGrenadeTimer)))
    (:else)))

(event EventDropLethal
  (bind _cookgrenadetimer (Variables|Default|GetCookGrenadeTimer))
  ;[0 0 0] Drop lethal
  (Variables|Default|SetbReleased true)
  (if (Utilities|Time|IsTimerActivebyHandle _cookgrenadetimer)
    (CallFunction|ServerSpawnGrenade (Utilities|Time|GetTimerRemainingTimebyHandle _cookgrenadetimer) (Transformation|GetWorldLocation (Variables|Default|GetTPP_Mesh)))
    (Utilities|Time|ClearandInvalidateTimerbyHandle _cookgrenadetimer)))

(fn ConstructionScript
  (|CallParentFunction))