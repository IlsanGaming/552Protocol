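; Timed target trial minigame actor that a player starts at a box trigger, hitting staged targets on the way to an end trigger.
; Overlapping triggers advance the stage and activate its targets, whose hit events update the WB_TrialInfo HUD.
; Tick accumulates time while a looping timer refreshes the display.
; Finishing adds a penalty per missed target, shows results and saves the best time to a SaveGame slot.
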(event OnComponentBeginOverlap(StartTrialTrigger)
  (params (OverlappedComponent :type Primitive%20Component%20Object%20Reference) (OtherActor :type Actor%20Object%20Reference) (OtherComp :type Primitive%20Component%20Object%20Reference) (OtherBodyIndex :type Integer) (bFromSweep :type Boolean) (SweepResult :type Hit%20Result%20Structure%20%28by%20ref%29))
  ;[0 0 0] Overlap Triggers
  ;;[0 0 0] On Overlap Start Trigger
  (bind _aspawn (Utilities|Casting|CastToPawn OtherActor))
  (if (not (Pawn|IsBotControlled _aspawn))
    (if (Variables|Default|GetTrialInProgress)
      (CallFunction|ResetTrial)
      (else
        (CallFunction|StartTrial)
        (Collision|SetCollisionEnabled (Variables|Default|GetStartTrialTrigger) "NoCollision")))))

(event OnActorBeginOverlap(EndTrigger)
  (params (OverlappedActor :type Actor%20Object%20Reference) (OtherActor :type Actor%20Object%20Reference))
  ;[0 0 0] Overlap Triggers
  ;;[0 0 0] Reset and End Trigger
  (CallFunction|FinishTrial))

(event OnActorBeginOverlap(ResetTrigger)
  (params (OverlappedActor :type Actor%20Object%20Reference) (OtherActor :type Actor%20Object%20Reference))
  ;[0 0 0] Overlap Triggers
  ;;[0 0 0] Reset and End Trigger
  (CallFunction|ResetTrial))

(event Custom|Reset_Trial
  (bind _wb_trial (Variables|Default|GetWB_Trial))
  ;[0 0 0] Reset Trial
  (Variables|Default|SetCurrentTrialStage 0)
  (Variables|Default|SetTrialInProgress false)
  (Utilities|IsValid _wb_trial
    (:Is%20Valid
      (Widget|RemovefromParent _wb_trial))
    (:Is%20Not%20Valid
      _))
  (if (Utilities|Array|IsValidIndex (Variables|Default|GetTargetsList))
    (for _array_element (Variables|Default|GetTargetsList)
      (Default|ResetDummyPosition _array_element))
    (Collision|SetCollisionEnabled (Variables|Default|GetStartTrialTrigger) "QueryOnly")
    (Actor|Tick|SetActorTickEnabled false) ; Stops the time
    (Utilities|Time|ClearandInvalidateTimerbyHandle (Variables|Default|GetTimerHandle))
    (Collision|SetCollisionEnabled (Variables|Default|GetStartTrialTrigger) "QueryOnly")
    (for _array_element_2 (Variables|Default|GetTriggersList)
      (EventDispatchers|UnbindallEventsfromOnActorBeginOverlap _array_element_2))))

(event Custom|FinishTrial
  ;[0 0 0] Finish Trial
  (if (Variables|Default|GetTrialInProgress)
    (Actor|Tick|SetActorTickEnabled false)
    (Utilities|Time|ClearandInvalidateTimerbyHandle (Variables|Default|GetTimerHandle))
    (bind _output_get (Variables|Default|SetPenalization (Math|Conversions|ToFloat(Integer) (* (- (Variables|Default|GetTrialTotalTargets) (Variables|Default|GetTargetsHitted)) 3))))
    (bind _output_get_2 (Variables|Default|SetFinalTime (+ (Variables|Default|GetTime) _output_get)))
    (bind _output_get_3 (Variables|Default|SetbNewRecord (< _output_get_2 (Variables|Default|GetCurrentRecordTime))))
    (if _output_get_3
      (CallFunction|SaveNewTrialRecord _output_get_2))
    (Default|ShowResults (Variables|Default|GetWB_Trial) (Variables|Default|GetCurrentRecordTime) (Variables|Default|GetFinalTime) (Variables|Default|GetPenalization))
    (Collision|SetCollisionEnabled (Variables|Default|GetStartTrialTrigger) "QueryOnly")))

(event Custom|NextStage
  (bind _targetslist (Variables|Default|GetTargetsList))
  ;[0 0 0] Next Trial Stage
  (if (Utilities|Array|IsValidIndex _targetslist)
    (for _array_element _targetslist
      (if (== (Variables|/Game/FPS_Controller/Blueprints/DummyTarget/BP_Base_Target.BP_Base_Target_C|GetTrial_Stage _array_element) (Variables|Default|GetCurrentTrialStage))
        (Default|InitTarget _array_element)
        (EventDispatchers|AssignOnHit _array_element (delegate Custom|OnHit_Event))))))

(event Custom|OnHit_Event
  (params (TimeLeft :type Float%20%28double-precision%29))
  ;[0 0 0] Next Trial Stage
  (bind _output_get (Variables|Default|SetTargetsHitted (+ (Variables|Default|GetTargetsHitted) 1)))
  (bind _wb_trial (Variables|Default|GetWB_Trial)
    (:then
      (Default|UpdateTargets _wb_trial _output_get (Variables|Default|GetTrialTotalTargets)))
    (:else)))

(event Custom|StartTrial
  ;[0 0 0] Start Trial
  (CallFunction|LoadRecord)
  (bind _returnvalue (Utilities|Time|SetTimerbyEvent (delegate Custom|UpdateTimer) 0.1 true))
  (Variables|Default|SetTimerHandle _returnvalue)
  (Variables|Default|SetTrialTotalTargets (Utilities|Array|Length (Variables|Default|GetTargetsList)))
  (Variables|Default|SetTargetsHitted 0)
  (Variables|Default|SetTime 0.0)
  (Actor|Tick|SetActorTickEnabled true) ; Stats The timer
  (Variables|Default|SetTrialInProgress true)
  (Utilities|FlowControl|Sequence
    (:then_0
      ;;[0.07292 0.07292 0.07292] Show Widget
      (Utilities|IsValid (Variables|Default|GetWB_Trial)
        (:Is%20Valid
          (Widget|RemovefromParent (Variables|Default|GetWB_Trial)))
        (:Is%20Not%20Valid
          _))
      (bind _returnvalue_2 (UserInterface|CreateWidget "/Game/FPS_Controller/UI/Trial/WB_TrialInfo.WB_TrialInfo_C" (Game|GetPlayerController 0)))
      (bind _output_get (Variables|Default|SetWB_Trial _returnvalue_2))
      (UserInterface|Viewport|AddtoViewport _output_get 0)
      (Default|UpdateTargets (Variables|Default|GetWB_Trial) 0 (Variables|Default|GetTrialTotalTargets)))
    (:then_2
      (Variables|Default|SetCurrentTrialStage 1)
      (CallFunction|NextStage))
    (:then_3
      (for _array_element (Variables|Default|GetTriggersList)
        (Collision|SetActorEnableCollision _array_element true)
        (Collision|BindEventtoOnActorBeginOverlap _array_element (delegate Custom|OnTriggerOverlap))))))

(event Custom|OnTriggerOverlap
  (params (OverlappedActor :type Actor%20Object%20Reference) (OtherActor :type Actor%20Object%20Reference))
  ;[0 0 0] Overlap Triggers
  (bind _astrigger_base (Utilities|Casting|CastToTriggerBase OverlappedActor))
  (Math|Integer|IncrementInt (Variables|Default|GetCurrentTrialStage)
    (:%20%20
      (CallFunction|NextStage)
      (Collision|SetActorEnableCollision _astrigger_base false))))

(event Custom|UpdateTimer
  ;[0 0 0] Start Trial
  (Default|UpdateTime (Variables|Default|GetWB_Trial) (Variables|Default|GetTime)))

(event EventTick
  (params (DeltaSeconds :type Float%20%28single-precision%29))
  ;[0 0 0] Tick
  (Variables|Default|SetTime (+ (Variables|Default|GetTime) DeltaSeconds)))

(fn ConstructionScript
  (Components|Box|SetBoxExtent (Variables|Default|GetStartTrialTrigger) (Variables|Default|GetStartTriggerExtent) true))

(fn OpenTrialWidget)

(fn SaveNewTrialRecord
  (params (RecordTime :type Float%20%28double-precision%29))
  (bind _returnvalue (SaveGame|CreateSaveGameObject "/Game/FPS_Controller/Blueprints/SaveGame/BP_Trial_ScoreSave.BP_Trial_ScoreSave_C"))
  (bind _output_get (Variables|/Game/FPS_Controller/Blueprints/SaveGame/BP_Trial_ScoreSave.BP_Trial_ScoreSave_C|SetRecordTime _returnvalue RecordTime))
  (Variables|Default|SetCurrentRecordTime _output_get)
  (SaveGame|SaveGametoSlot _returnvalue "Save"))

(fn LoadRecord
  (bind _returnvalue (SaveGame|LoadGamefromSlot "Save"))
  (bind _asbp_trial_score_save (Utilities|Casting|CastToBP_Trial_ScoreSave _returnvalue)
    (:then
      (Variables|Default|SetCurrentRecordTime (Variables|/Game/FPS_Controller/Blueprints/SaveGame/BP_Trial_ScoreSave.BP_Trial_ScoreSave_C|GetRecordTime _asbp_trial_score_save)))
    (:CastFailed
      (SaveGame|CreateSaveGameObject "/Game/FPS_Controller/Blueprints/SaveGame/BP_Trial_ScoreSave.BP_Trial_ScoreSave_C")
      (Variables|Default|SetCurrentRecordTime 5e+03))))